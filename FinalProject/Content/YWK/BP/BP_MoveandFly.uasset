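; BP_MoveandFly is an actor Blueprint with a clickable MeshComp, but all of its events and its construction script are empty, so it adds no behavior.
; Disconnected event-graph nodes hold drafts of a toggled outline overlay material and a WBP_Choice widget added to the viewport.
; Disconnected construction-script nodes draft a dynamic outline material with custom line thickness and movement control points, none of which run.
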(event OnClicked(meshComp)
  (params (TouchedComponent :type Primitive%20Component%20Object%20Reference) (ButtonPressed :type Key%20Structure :default "None")))

(event EventBeginPlay)

(event Collision|EventActorBeginOverlap
  (params (OtherActor :type Actor%20Object%20Reference)))

(event EventTick
  (params (DeltaSeconds :type Float%20%28single-precision%29)))

(fn ConstructionScript)